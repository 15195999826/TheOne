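; Base character Blueprint for a turn-based game, handling selection, turn and death visual feedback.
; Selection events toggle a decal, while turn events show or hide an active-tip mesh that starts hidden.
; Setting the camp binds the head bar widget to the AbilitySystemComponent and flags whether it is the player's.
; Death hides the tip, then after a delay hides and unbinds the head bar; a ragdoll death sequence is left unconnected.
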(event EventBeginPlay
  (Development|SetHiddeninGame (Variables|Default|GetActiveTIpStaticMesh) true false))

(event Collision|EventActorBeginOverlap
  (params (OtherActor :type Actor%20Object%20Reference)))

(event EventTick
  (params (DeltaSeconds :type Float%20%28single-precision%29)))

(event EventOnGetTurn
  (Development|SetHiddeninGame (Variables|Default|GetActiveTIpStaticMesh) false false))

(event EventOnDeselected
  (Rendering|SetVisibility (Variables|Default|GetSelectDecal) false false))

(event EventOnSelected
  (Rendering|SetVisibility (Variables|Default|GetSelectDecal) true false))

(event EventOnSetCamp
  (params (InCamp :type ETheOneCamp%20Enum :default "None"))
  (CallFunction|SetUpHeadBar InCamp))

(event EventDie
  (Development|SetHiddeninGame (Variables|Default|GetActiveTIpStaticMesh) true false)
  (Utilities|FlowControl|Delay 1.5)
  (Development|SetHiddeninGame (Variables|Default|GetHeadBarWidgetComponent) true false)
  (bind _aswbp_character_head_bar (Utilities|Casting|CastToWBP_CharacterHeadBar (UserInterface|GetWidget (Variables|Default|GetHeadBarWidgetComponent))))
  (Class|CharacterHeadBar|UnBind _aswbp_character_head_bar))

(event EventOnEndTurn
  (Development|SetHiddeninGame (Variables|Default|GetActiveTIpStaticMesh) true false))

(fn ConstructionScript)

(fn SetUpHeadBar
  (params (Selection :type ETheOneCamp%20Enum :default "None"))
  (bind _aswbp_character_head_bar (Utilities|Casting|CastToWBP_CharacterHeadBar (UserInterface|GetWidget (Variables|Default|GetHeadBarWidgetComponent))))
  (bind _output_get (LocalVariables|SetHeadBar _aswbp_character_head_bar))
  (Class|CharacterHeadBar|Bind _output_get (Variables|Default|GetAbilitySystemComponent))
  (switch Utilities|FlowControl|Switch|SwitchonETheOneCamp Selection
    (:None
      (Variables|/Game/Blueprints/UI/Component/WBP_CharacterHeadBar.WBP_CharacterHeadBar_C|SetIsForPlayer (LocalVariables|GetHeadBar) false :!label _label))
    (:Player
      (Variables|/Game/Blueprints/UI/Component/WBP_CharacterHeadBar.WBP_CharacterHeadBar_C|SetIsForPlayer (LocalVariables|GetHeadBar) true))
    (:Enemy
      (goto _label))
    (:Neutral
      (goto _label))))