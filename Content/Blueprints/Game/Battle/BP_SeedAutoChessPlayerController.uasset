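; BP_SeedAutoChessPlayerController is the player controller Blueprint for the auto chess battle, adding an editor-only level-edit toggle.
; During Play In Editor, Shift+E flips the EditLevel flag, creating and showing a new WBP_LevelEdit widget or hiding and removing the existing one.
; BeginPlay, Tick and the construction script are empty, and a cheat manager check is left unconnected.
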(event EventBeginPlay)

(event EventTick
  (params (DeltaSeconds :type Float%20%28single-precision%29)))

(event Input|KeyboardEvents|ShiftE
  (params (Key :type Key%20Structure))
  (:Pressed
    (if (Class|TheOneHexMapPlayerController|IsPlayinEditor)
      (bind _isa (Utilities|FlowControl|FlipFlop)
        (:A
          _)
        (:B
          _))
      (Variables|Default|SetEditLevel _isa)
      (if (Variables|Default|GetEditLevel)
        (bind _returnvalue (UserInterface|CreateWidget "/Game/Blueprints/UI/WBP_LevelEdit.WBP_LevelEdit_C"))
        (bind _output_get (Variables|Default|SetEditUI _returnvalue))
        (UserInterface|Viewport|AddtoViewport _output_get 0)
        (Default|OnEdit (Variables|Default|GetEditUI))
        (else
          (Utilities|IsValid (Variables|Default|GetEditUI)
            (:Is%20Valid
              (Default|OnHide (Variables|Default|GetEditUI))
              (Widget|RemovefromParent (Variables|Default|GetEditUI)))))))))

(fn ConstructionScript)