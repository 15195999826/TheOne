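; Player controller for HexAXELand that turns cursor hit events into AI orders for the selected character and updates the cursor widget.
; Right-clicks on walkable ground send the character's AI controller a target location, or a target actor if a hex-interface actor stands there.
; Hit hex actors set the cursor's camp to neutral, player or enemy relative to the selected character, and right-clicking targets them.
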(event EventBeginPlay
  (bind _foundwidgets (Widget|GetAllWidgetsOfClass "/Game/Blueprints/UI/WBP_Seed_Cursor.WBP_Seed_Cursor_C" false))
  (Variables|Default|SetSeedCuror (Utilities|Array|Get(acopy) _foundwidgets)))

(event EventTick
  (params (DeltaSeconds :type Float%20%28single-precision%29)))

(event EventOnHitGround
  (params (HitLocation :type Vector%20%28by%20ref%29 :default "0, 0, 0") (bIsRightClick :type Boolean) (CanWalk :type Boolean))
  (Default|SetCamp (Variables|Default|GetSeedCuror) "None")
  (if bIsRightClick
    (if CanWalk
      (Utilities|IsValid (Variables|Default|GetSelectedCharacter)
        (:Is%20Valid
          (bind _returnvalue (Class|TheOneAutoChessBPFunctionLibrary|HasActorStandingonGrid HitLocation)
            (:Valid
              (if (Utilities|DoesObjectImplementInterface _returnvalue "/Script/TheOne.InHexActorInterface")
                (CallFunction|OnHitinHexActor _returnvalue true)
                (else
                  (Class|TheOneAICommandInterface|SetAITargetLocation(Message) (Pawn|GetController (Variables|Default|GetSelectedCharacter)) HitLocation :!label _label))))
            (:Invalid
              (goto _label))))))))

(event EventOnCursorStateChange
  (params (InState :type ETheOneCursorState%20Enum :default "Normal") (InSelectActorType :type ETheOneSelectActorType%20Enum :default "Any") (InReleaseDistance :type Integer))
  (Default|SetCursorState (Variables|Default|GetSeedCuror) InState))

(event EventOnHitActor
  (params (InHitActor :type Actor%20Object%20Reference) (bIsRightClick :type Boolean))
  (if (Utilities|DoesObjectImplementInterface InHitActor "/Script/TheOne.InHexActorInterface")
    (CallFunction|OnHitinHexActor InHitActor bIsRightClick)))

(fn ConstructionScript
  (|CallParentFunction))

(fn OnHitinHexActor
  (params (InHitActor :type Actor%20Object%20Reference) (IsRightClick :type Boolean))
  (bind _selectedcharacter (Variables|Default|GetSelectedCharacter))
  (bind _returnvalue (Class|InHexActorInterface|GetCamp(Message) InHitActor))
  (LocalVariables|SetHitActorCamp _returnvalue)
  (Utilities|FlowControl|Sequence
    (:then_0
      (if (Utilities|Enum|Equal(Enum) (LocalVariables|GetHitActorCamp) "Neutral")
        (LocalVariables|SetCurrentTemp "Neutral")
        (else
          (Utilities|IsValid _selectedcharacter
            (:Is%20Valid
              (if (Utilities|Enum|Equal(Enum) (Variables|/Script/TheOne.TheOneCharacterBase|GetCamp _selectedcharacter) (LocalVariables|GetHitActorCamp))
                (LocalVariables|SetCurrentTemp "Player")
                (else
                  (LocalVariables|SetCurrentTemp "Enemy"))))
            (:Is%20Not%20Valid
              (LocalVariables|SetCurrentTemp "Neutral"))))))
    (:then_1
      (Default|SetCamp (Variables|Default|GetSeedCuror) (LocalVariables|GetCurrentTemp)))
    (:then_2
      (if IsRightClick
        (Utilities|IsValid (Variables|Default|GetSelectedCharacter)
          (:Is%20Valid
            (Class|TheOneAICommandInterface|SetAITargetActor(Message) (Pawn|GetController (Variables|Default|GetSelectedCharacter)) InHitActor)))))))