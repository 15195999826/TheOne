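; BP_Battle reacts to battle stage changes, extending the parent's stage-change handling with UI and visual feedback.
; On a pending new round, it notifies WBP_BattleWindow of the round, waits briefly, then completes the wait signal.
; On a character turn, it reveals the active-tip mesh on the acting BP_SeedCharacterBase from the action queue.
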(event EventOnBattleStageChanged
  (bind _battlecontext (Variables|Default|GetBattleContext))
  (bind (_stage _round _currentturn _actionqueue) (Utilities|Struct|BreakTheOneBattleContext _battlecontext))
  (|CallParentFunction)
  (switch Utilities|FlowControl|Switch|SwitchonETheOneBattleStage _stage
    (:NewRoundPending
      (bind _aswbp_battle_window (Utilities|Casting|CastToWBP_BattleWindow (Class|TheOneBattle|GetBattleWindow)))
      (Default|OnNewRoundPending _aswbp_battle_window _round)
      (Utilities|FlowControl|Delay 2.0)
      (Class|TheOneBattle|CompleteWaitSignal))
    (:CharacterTurn
      (bind _asbp_seed_character_base (Utilities|Casting|CastToBP_SeedCharacterBase (Utilities|Array|Get(acopy) _actionqueue _currentturn)))
      (Development|SetHiddeninGame (Variables|/Game/Blueprints/Pawn/Character/BP_SeedCharacterBase.BP_SeedCharacterBase_C|GetActiveTIpStaticMesh _asbp_seed_character_base) false false))))

(fn ConstructionScript)