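; GM_CharacterOverview is a game mode that lays out the configured characters in a grid for an overview.
; On BeginPlay it walks every row name in DT_ChracterTemplateTable and spawns an AI pawn for each one that passes IsCharacterConfigValid.
; Each pawn joins the Player camp under a deprecated default AI controller.
; Grid cells derive from the row index in tens, offset from StartPosition, so invalid rows leave gaps.
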(event EventBeginPlay
  (bind _outrownames (DataTable|GetDataTableRowNames "/Game/Blueprints/Data/DT_ChracterTemplateTable.DT_ChracterTemplateTable"))
  (for (_array_element _array_index) _outrownames
    (if (Class|TheOneBlueprintFunctionLibrary|IsCharacterConfigValid _array_element)
      (Class|TheOneGameModeBase|SpawnOneAIatTransform "/Game/Blueprints/AI/Deprecated_DefaultAI/BP_Seed_Deprecated_DefaultAI.BP_Seed_Deprecated_DefaultAI_C" (Math|Transform|MakeTransform (+ (Variables|Default|GetStartPosition) (Math|Vector|MakeVector (* (Math|Integer|%(Integer) _array_index 10) 150) (* (/ _array_index 10) 150) 0.0)) "0.000000,90.000000,0.000000") (Utilities|Struct|MakeTheOneAIPawnSpawnInfo "None" _array_element "None" 0)))))

(event EventTick
  (params (DeltaSeconds :type Float%20%28single-precision%29)))

(fn ConstructionScript)