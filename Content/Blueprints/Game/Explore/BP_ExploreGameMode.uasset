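; BP_ExploreGameMode is the game mode for exploration levels, handling the screen transition and initial AI spawn.
; BeginPlay shows the game instance's transition; when the level is prepared, it spawns one AI by spawn-info start tag and then transitions out.
; An unconnected chain would spawn a BP_BattleTrigger at a fixed hex-grid cell, but it never runs.
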(event EventBeginPlay
  (bind _gi (CallFunction|GetBPSeedGameInstance))
  (Default|ShowTransition _gi))

(event EventTick
  (params (DeltaSeconds :type Float%20%28single-precision%29)))

(event EventOnLevelPrepared
  (Class|TheOneGameModeBase|SpawnOneAI 0 (Utilities|Struct|MakeTheOneAIPawnSpawnInfo "None" "None" "10001"))
  (bind _gi (CallFunction|GetBPSeedGameInstance))
  (Default|TransitionOut _gi))

(fn ConstructionScript)