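; Deprecated RTS-style player controller that caches the seed cursor widget on BeginPlay and receives ground and character hit events.
; Both hit handlers are effectively empty, with the character event forwarding to a stub function.
; Disconnected logic remains for setting the cursor's camp and sending right-click target location or actor messages to the selected character's AI controller, but it never runs.
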(event EventBeginPlay
  (bind _foundwidgets (Widget|GetAllWidgetsOfClass "/Game/Blueprints/UI/WBP_Seed_Cursor.WBP_Seed_Cursor_C" false))
  (Variables|Default|SetSeedCuror (Utilities|Array|Get(acopy) _foundwidgets)))

(event EventTick
  (params (DeltaSeconds :type Float%20%28single-precision%29)))

(event EventOnHitGround
  (params (HitLocation :type Vector%20%28by%20ref%29 :default "0, 0, 0") (bIsRightClick :type Boolean)))

(event EventOnHitCharacter
  (params (HitCharacter :type The%20One%20Character%20Base%20Object%20Reference) (bIsRightClick :type Boolean))
  (CallFunction|OnHitCharacter HitCharacter bIsRightClick))

(fn ConstructionScript
  (|CallParentFunction))

(fn OnHitCharacter
  (params (HitCharacter :type The%20One%20Character%20Base%20Object%20Reference) (IsRightClick :type Boolean)))