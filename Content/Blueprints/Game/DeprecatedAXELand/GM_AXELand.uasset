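; AXELand game mode, in a deprecated folder, for a character sandbox where the player character is swapped and others are spawned or deleted.
; BeginPlay pushes the main widget and binds its events.
; Swapping respawns a config AI at the old pawn's location; spawning picks random navigable points near it.
; Deletion skips the player's pawn; teammate and enemy spawns both resolve to camp value 0.
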(event EventBeginPlay
  (Utilities|FlowControl|Sequence
    (:then_0
      (bind _returnvalue (UserInterface|CreateWidget "/Game/Blueprints/UI/AXELand/WBP_AXELand_Main.WBP_AXELand_Main_C"))
      (Utilities|FlowControl|Sequence
        (:then_0
          (EventDispatchers|BindEventtoOnPlayerCharacterChange _returnvalue (EventDispatchers|CreateEvent :!event ChangePlayerCharacter)))
        (:then_1
          (EventDispatchers|BindEventtoOnSpawnCharacterChange _returnvalue (EventDispatchers|CreateEvent :!event ChangeSpawnCharacter)))
        (:then_2
          (EventDispatchers|BindEventtoOnSpawnEnemy _returnvalue (EventDispatchers|CreateEvent :!event SpawnEnemy)))
        (:then_3
          (EventDispatchers|BindEventtoOnSpawnPlayerTeammate _returnvalue (EventDispatchers|CreateEvent :!event SpawnPlayer)))
        (:then_4
          (EventDispatchers|BindEventtoOnDeleteSelectedCharacter _returnvalue (EventDispatchers|CreateEvent :!event DeleteSelectedCharacter)))
        (:then_5
          (Class|TheOneBlueprintFunctionLibrary|PushUI "BackEnd" _returnvalue "HAlign_Fill" "VAlign_Fill"))))
    (:then_1
      (Class|TheOneBlueprintFunctionLibrary|DisableUINav))))

(event EventTick
  (params (DeltaSeconds :type Float%20%28single-precision%29)))

(fn ConstructionScript)

(fn ChangePlayerCharacter
  (params (OutRowName :type Name))
  (Utilities|FlowControl|Sequence
    (:then_0
      (Utilities|IsValid (Variables|Default|GetPlayerCharacterCtrl)
        (:Is%20Valid
          (Utilities|IsValid (Pawn|GetControlledPawn (Variables|Default|GetPlayerCharacterCtrl))
            (:Is%20Valid
              (LocalVariables|SetCachedLocation (Transformation|GetActorLocation (Pawn|GetControlledPawn (Variables|Default|GetPlayerCharacterCtrl)))))))))
    (:then_1
      (Utilities|IsValid (Variables|Default|GetPlayerCharacterCtrl)
        (:Is%20Valid
          (Class|TheOneGameModeBase|RemoveOneAI (Variables|Default|GetPlayerCharacterCtrl)))))
    (:then_2
      (bind _returnvalue (Class|TheOneGameModeBase|SpawnOneConfigAIatTransform (Math|Transform|MakeTransform (LocalVariables|GetCachedLocation)) (Utilities|Struct|MakeTheOneAIPawnSpawnInfo "None" OutRowName "None" 0)))
      (Variables|Default|SetPlayerCharacterCtrl _returnvalue))))

(fn ChangeSpawnCharacter
  (params (OutRowName :type Name))
  (Variables|Default|SetSpawnCharacterRow OutRowName))

(fn SpawnNewCharacter
  (params (IsPlayerTeammate :type Boolean))
  (bind _playercharacterctrl (Variables|Default|GetPlayerCharacterCtrl))
  (bind _returnvalue (Pawn|GetControlledPawn _playercharacterctrl))
  (if (not (== (Variables|Default|GetSpawnCharacterRow) ""))
    (Utilities|FlowControl|Sequence
      (:then_0
        (Utilities|IsValid (Variables|Default|GetPlayerCharacterCtrl)
          (:Is%20Valid
            (Utilities|IsValid _returnvalue
              (:Is%20Valid
                (LocalVariables|SetOrigin (Transformation|GetActorLocation _returnvalue)))))))
      (:then_1
        (bind (_randomlocation _returnvalue_2) (Class|NavigationSystemV1|GetRandomLocationinNavigableRadius (LocalVariables|GetOrigin) 5e+02 (Variables|Default|GetNav%20Data) 0))
        (if _returnvalue_2
          (Class|TheOneGameModeBase|SpawnOneConfigAIatTransform (Math|Transform|MakeTransform (+ _randomlocation "0.000000,0.000000,100.000000")) (Utilities|Struct|MakeTheOneAIPawnSpawnInfo (Utilities|Enum|ByteToEnumETheOneCamp (select IsPlayerTeammate 0 0)) (Variables|Default|GetSpawnCharacterRow) "None"))
          (else
            (Development|PrintText "无法随机地点")))))))

(fn SpawnPlayer
  (Spawn|SpawnNewCharacter true))

(fn DeleteSelectedCharacter
  (bind _playercharacterctrl (Variables|Default|GetPlayerCharacterCtrl))
  (bind _returnvalue (Pawn|GetControlledPawn _playercharacterctrl))
  (bind _asthe_one_player_controller_base (Utilities|Casting|CastToTheOnePlayerControllerBase (Game|GetPlayerController 0)))
  (LocalVariables|SetTempCharacter (Variables|/Script/TheOne.TheOnePlayerControllerBase|GetSelectedCharacter _asthe_one_player_controller_base))
  (Utilities|FlowControl|Sequence
    (:then_0
      (Utilities|IsValid (Variables|Default|GetPlayerCharacterCtrl)
        (:Is%20Valid
          (Utilities|IsValid _returnvalue
            (:Is%20Valid
              (if (== (LocalVariables|GetTempCharacter) _returnvalue)
                (return)))))))
    (:then_1
      (Class|TheOneGameModeBase|RemoveOneAICharacter (LocalVariables|GetTempCharacter)))))

(fn SpawnEnemy
  (Spawn|SpawnNewCharacter false))