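; BP_T generates a procedural landmass mesh in its construction script using Geometry Script on a dynamic mesh component.
; It places LandCount tapered cones at cellular FastNoise offsets, recording SpawnPoints and printing debug values.
; The combined mesh is voxel-solidified to merge overlaps, smoothed, plane-cut into a flat slab and given planar UVs.
; Event graph events are disabled, and the box-base nodes are disconnected.
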(event EventBeginPlay)

(event Collision|EventActorBeginOverlap
  (params (OtherActor :type Actor%20Object%20Reference)))

(event EventTick
  (params (DeltaSeconds :type Float%20%28single-precision%29)))

(fn ConstructionScript
  (bind _radius (Variables|Default|GetRadius))
  (bind _returnvalue (Game|ConstructObjectfromClass "/Script/FastNoiseGenerator.FastNoiseWrapper"))
  (bind _output_get (Variables|Default|SetNoise _returnvalue))
  (Class|FastNoiseWrapper|SetupFastNoise _output_get "Cellular" 133 0.5 "Quintic" "FBM" 3 2.0 0.5 0.45 "Natural" "Distance2")
  (bind _returnvalue_2 (DynamicMeshComponent|GetDynamicMesh (Variables|DynamicMeshActor|GetDynamicMeshComponent)))
  (bind _output_get_2 (Variables|Default|SetDynMesh _returnvalue_2))
  (DynamicMesh|Reset _output_get_2)
  (Utilities|Array|Clear (Variables|Default|GetSpawnPoints))
  (Utilities|FlowControl|Sequence
    (:then_0
      (for _index (range 0 (Variables|Default|GetLand%20Count))
        (Development|PrintString (Utilities|String|ToString(Text) (Utilities|Text|FormatText "x:{x},y: {y}, Jitter:{Jitter}" (Class|FastNoiseWrapper|GetNoise2D (Variables|Default|GetNoise) (Math|Conversions|ToFloat(Integer) (/ _index 4)) (Math|Conversions|ToFloat(Integer) (/ _index 4))) (Class|FastNoiseWrapper|GetNoise2D (Variables|Default|GetNoise) (Math|Conversions|ToFloat(Integer) _index) (Math|Conversions|ToFloat(Integer) _index)) (Class|FastNoiseWrapper|GetCellularJitter (Variables|Default|GetNoise)))))
        (Utilities|Array|Add :TargetArray (Variables|Default|GetSpawnPoints))
        (bind _returnvalue_3 (Class|GeometryScriptLibraryMeshPrimitiveFunctions|AppendCone :TargetMesh (Variables|Default|GetDynMesh) :Transform (Math|Transform|MakeTransform (Math|Vector|MakeVector (* (Class|FastNoiseWrapper|GetNoise2D (Variables|Default|GetNoise) (Math|Conversions|ToFloat(Integer) (/ _index 4)) (Math|Conversions|ToFloat(Integer) (/ _index 4))) 1.5e+02) (* (Class|FastNoiseWrapper|GetNoise2D (Variables|Default|GetNoise) (Math|Conversions|ToFloat(Integer) _index) (Math|Conversions|ToFloat(Integer) _index)) 1.5e+02) 0.0)) :BaseRadius _radius :TopRadius (/ _radius 1.5) :Height 8e+02 :RadialSteps 32 :HeightSteps 1 :Debug 0))
        (Class|GeometryScriptLibraryMeshBooleanFunctions|ApplyMeshPlaneSlice :TargetMesh _returnvalue_3 :Options (Utilities|Struct|MakeGeometryScriptMeshPlaneSliceOptions true true 0.01 1.0) :Debug 0)))
    (:then_1
      ;[1 1 1] 接触到的Mesh会被合并，体素化，网格化
      (bind _returnvalue_4 (Class|GeometryScriptLibraryMeshVoxelFunctions|ApplyMeshSolidify (Variables|Default|GetDynMesh) (Utilities|Struct|MakeGeometryScriptSolidifyOptions (Utilities|Struct|MakeGeometryScript3DGridParameters "GridResolution" 0.25 64) 0.2 true 0.0 4) 0))
      (bind _returnvalue_5 (Class|GeometryScriptLibraryMeshNormalsFunctions|SetPerVertexNormals _returnvalue_4 0))
      (bind _returnvalue_6 (Class|GeometryScriptLibraryMeshDeformFunctions|ApplyIterativeSmoothingtoMesh :TargetMesh _returnvalue_5 :Options (Utilities|Struct|MakeGeometryScriptIterativeMeshSmoothingOptions 6 0.2 "FullMeshSelection") :Debug 0)) ; 平滑
      (bind _returnvalue_7 (Class|GeometryScriptLibraryMeshSubdivideFunctions|ApplyPNTessellation :TargetMesh _returnvalue_6 :TessellationLevel 0 :Debug 0)) ; 让面更多
      (bind _returnvalue_8 (Class|GeometryScriptLibraryMeshBooleanFunctions|ApplyMeshPlaneCut _returnvalue_7 (Math|Transform|MakeTransform "0.000000,0.000000,-50.000000" "0.000000,0.000000,180.000000") (Utilities|Struct|MakeGeometryScriptMeshPlaneCutOptions false false false 1.0) 0)) ; 裁剪
      (bind _returnvalue_9 (Class|GeometryScriptLibraryMeshBooleanFunctions|ApplyMeshPlaneCut :TargetMesh _returnvalue_8 :CutFrame (Math|Transform|MakeTransform "0.000000,0.000000,10.000000") :Debug 0))
      (Class|GeometryScriptLibraryMeshUVFunctions|SetMeshUVsfromPlanarProjection :TargetMesh _returnvalue_9 :PlaneTransform (Math|Transform|MakeTransform "0, 0, 0" "0, 0, 0" "100.000000,100.000000,100.000000") :Debug 0))))