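; Geometry Script test actor that procedurally builds two offset hexagonal tiles with a hole in its DynamicMeshComponent from the construction script.
; AddHex trims a box with four plane cuts and boolean-unions it into the reset mesh.
; AddHole then subtracts a tapered cone at a fixed-seed random point, and a grid-based solidify pass finishes the result.
; Compute meshes are allocated but never released on the live path.
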(event EventBeginPlay)

(event Collision|EventActorBeginOverlap
  (params (OtherActor :type Actor%20Object%20Reference)))

(event EventTick
  (params (DeltaSeconds :type Float%20%28single-precision%29)))

(fn ConstructionScript
  (bind _returnvalue (DynamicMeshComponent|GetDynamicMesh (Variables|DynamicMeshActor|GetDynamicMeshComponent)))
  (bind _output_get (Variables|Default|SetDynMesh _returnvalue))
  (DynamicMesh|Reset _output_get)
  (CallFunction|AddHex (Math|Transform|MakeTransform "0.000000,50.000000,0.000000"))
  (CallFunction|AddHex (Math|Transform|MakeTransform "0.000000,-100.000000,10.000000"))
  (CallFunction|AddHole)
  (Class|GeometryScriptLibraryMeshVoxelFunctions|ApplyMeshSolidify (Variables|Default|GetDynMesh) (Utilities|Struct|MakeGeometryScriptSolidifyOptions (Utilities|Struct|MakeGeometryScript3DGridParameters "GridResolution" 0.5 48) 0.5 true 1.0 3 true) 0))

(fn AddHole
  (bind _returnvalue (DynamicMeshActor|AllocateComputeMesh))
  (bind _returnvalue_2 (Class|GeometryScriptLibraryMeshPrimitiveFunctions|AppendCone :TargetMesh _returnvalue :Transform (Math|Conversions|ToTransform(Vector) (Class|KismetMathLibrary|RandomPointinBoundingBoxfromStream (Math|Random|MakeRandomStream 11) "0, 0, 0" "20.000000,20.000000,0.000000")) :BaseRadius 3e+01 :TopRadius 2e+01 :Height 5e+01 :Debug 0))
  (bind _returnvalue_3 (GeometryScript|Booleans|ApplyMeshBoolean :TargetMesh (Variables|Default|GetDynMesh) :ToolMesh _returnvalue_2 :Operation "Subtract" :Options (Utilities|Struct|MakeGeometryScriptMeshBooleanOptions true true 0.01 false) :Debug 0)))

(fn AddHex
  (params (Position :type Transform))
  (LocalVariables|SetNewLocalVar Position)
  (bind _returnvalue (DynamicMeshActor|AllocateComputeMesh))
  (bind _returnvalue_2 (Class|GeometryScriptLibraryMeshPrimitiveFunctions|AppendBox :TargetMesh _returnvalue :Transform (Math|Transform|MakeTransform "0, 0, 0") :DimensionX 173.3 :DimensionY 2e+02 :DimensionZ 5e+01 :Debug 0))
  (bind _returnvalue_3 (Class|GeometryScriptLibraryMeshBooleanFunctions|ApplyMeshPlaneCut :TargetMesh _returnvalue_2 :CutFrame (Math|Transform|MakeTransform "-43.300000,-75.000000,0.000000" "90.000000,60.000000,0.000000") :Debug 0))
  (bind _returnvalue_4 (Class|GeometryScriptLibraryMeshBooleanFunctions|ApplyMeshPlaneCut :TargetMesh _returnvalue_3 :CutFrame (Math|Transform|MakeTransform "43.300000,-75.000000,0.000000" "-90.000000,-60.000000,0.000000") :Debug 0))
  (bind _returnvalue_5 (Class|GeometryScriptLibraryMeshBooleanFunctions|ApplyMeshPlaneCut :TargetMesh _returnvalue_4 :CutFrame (Math|Transform|MakeTransform "43.300000,75.000000,0.000000" "-90.000000,60.000000,0.000000") :Debug 0))
  (bind _returnvalue_6 (Class|GeometryScriptLibraryMeshBooleanFunctions|ApplyMeshPlaneCut :TargetMesh _returnvalue_5 :CutFrame (Math|Transform|MakeTransform "-43.300000,75.000000,0.000000" "90.000000,-60.000000,0.000000") :Debug 0))
  (GeometryScript|Booleans|ApplyMeshBoolean :TargetMesh (Variables|Default|GetDynMesh) :ToolMesh _returnvalue_6 :ToolTransform (LocalVariables|GetNewLocalVar) :Operation "Union" :Debug 0))