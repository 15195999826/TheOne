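; Base actor for mouse-driven interactable objects, with hover highlighting and a toggleable interaction tip widget.
; Cursor hover calls focus hooks and toggles custom depth with a stencil value on static meshes under ModelRoot.
; Left and right clicks call separate hooks, and left click also shows or hides TipUI, which starts hidden.
; The tip widget's button calls OnInteractBase, while OnInteract only prints a placeholder message and the construction script is empty.
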(event Custom|OnClicked_Event
  (Class|TheOneInteractActor|OnInteractBase))

(event EventBeginPlay
  (Rendering|SetVisibility (Variables|Default|GetTipUI) false false)
  (bind _aswbp_item_interact_tips (Utilities|Casting|CastToWBP_Item_InteractTips (UserInterface|GetWidget (Variables|Default|GetTipUI))))
  (EventDispatchers|AssignOnClicked (Variables|/Game/Blueprints/UI/Component/WBP_Item_InteractTips.WBP_Item_InteractTips_C|GetButton_Interact _aswbp_item_interact_tips) (delegate Custom|OnClicked_Event)))

(event MouseInput|EventActorBeginCursorOver
  (Class|TheOneInteractActor|OnFocus)
  (for _array_element (Components|GetChildrenComponents (Variables|Default|GetModelRoot) false)
    (bind _asstatic_mesh_component (Utilities|Casting|CastToStaticMeshComponent _array_element))
    (Rendering|SetRenderCustomDepth _asstatic_mesh_component true)
    (Rendering|SetCustomDepthStencilValue _asstatic_mesh_component 250)))

(event MouseInput|EventActorEndCursorOver
  (Class|TheOneInteractActor|OnLoseFocus)
  (for _array_element (Components|GetChildrenComponents (Variables|Default|GetModelRoot) false)
    (bind _asstatic_mesh_component (Utilities|Casting|CastToStaticMeshComponent _array_element))
    (Rendering|SetRenderCustomDepth _asstatic_mesh_component false)))

(event MouseInput|EventActorOnClicked
  (params (ButtonPressed :type Key%20Structure))
  (bind _tipui (Variables|Default|GetTipUI))
  (if (== ButtonPressed "RightMouseButton")
    (Class|TheOneInteractActor|OnRightMouseButtonClick)
    (elif (== ButtonPressed "LeftMouseButton")
      (Class|TheOneInteractActor|OnLeftMouseButtonClick)
      (Rendering|SetVisibility _tipui (not (Rendering|IsVisible _tipui)) false))))

(event EventOnInteract
  (Development|PrintString "Hello"))

(fn ConstructionScript)