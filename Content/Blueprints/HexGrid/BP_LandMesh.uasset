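; BP_LandMesh builds a land mesh for a hex grid with Geometry Script, adding one tile per AddHex call.
; AddHex creates a box in a compute mesh, plane-cuts one corner, then boolean-unions it into DynMesh at the given center.
; The three cuts that would trim the other corners into a hexagon are disconnected and never run.
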(event EventBeginPlay)

(event Collision|EventActorBeginOverlap
  (params (OtherActor :type Actor%20Object%20Reference)))

(event EventTick
  (params (DeltaSeconds :type Float%20%28single-precision%29)))

(event EventAddHex
  (params (Center :type Vector%20%28by%20ref%29 :default "0, 0, 0") (Height :type Float%20%28single-precision%29) (HexRotator :type Rotator%20%28by%20ref%29 :default "0, 0, 0") (GridSize :type Float%20%28single-precision%29))
  (bind _returnvalue (DynamicMeshActor|AllocateComputeMesh))
  (bind _returnvalue_2 (Class|GeometryScriptLibraryMeshPrimitiveFunctions|AppendBox :TargetMesh _returnvalue :Transform (Math|Transform|MakeTransform "0, 0, 0") :DimensionX 173.3 :DimensionY 2e+02 :DimensionZ 5e+01 :Debug 0))
  (bind _returnvalue_3 (Class|GeometryScriptLibraryMeshBooleanFunctions|ApplyMeshPlaneCut _returnvalue_2 (Math|Transform|MakeTransform "-43.300000,-75.000000,0.000000" (Math|Rotator|MakeRotator 0.0 9e+01 6e+01)) (Utilities|Struct|MakeGeometryScriptMeshPlaneCutOptions true true false 1.0) 0))
  (GeometryScript|Booleans|ApplyMeshBoolean :TargetMesh (Variables|Default|GetDynMesh) :ToolMesh _returnvalue_3 :ToolTransform (Math|Conversions|ToTransform(Vector) Center) :Operation "Union" :Debug 0))

(fn ConstructionScript)