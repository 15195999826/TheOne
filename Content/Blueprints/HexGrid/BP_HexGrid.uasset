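; Hex grid actor Blueprint that adds debug overlays and broadcasts right-clicks with the hovered tile's row, column and world position.
; When the cheat manager allows it, a looping timer redraws debug text for all tiles, or only those within range of the cursor.
; H, C, R and D toggle cube coordinates, cost and occupancy, row/column, and cursor-only mode.
; Row/column labels convert cube to offset coordinates for flat-top or pointy-top non-radius grids.
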(event Custom|Event%20DebugDraws
  ;[1 1 1] Draw tiles Cube Debug
  (if (Math|Boolean|ORBoolean (Variables|Default|GetDebugCoords) (Variables|Default|GetDebugCost) (Variables|Default|GetDebugRowColumn))
    (if (Variables|Default|GetDebugCursorPoint)
      (bind _returnvalue (Class|HexGrid|WorldtoHex (Variables|Default|GetMouseHitLocation)))
      (bind _returnvalue_2 (Class|HexGrid|GetRange _returnvalue 2))
      (Variables|Default|SetDebugArray _returnvalue_2)
      (else
        (Variables|Default|SetDebugArray (Variables|Default|GetGridTiles))))
    (for _array_element (Variables|Default|GetDebugArray)
      (if (Variables|Default|GetDebugCoords)
        (CallFunction|DrawDebugCoords (.CubeCoord (Utilities|Struct|BreakHexTile _array_element)) (.WorldPosition (Utilities|Struct|BreakHexTile _array_element)) (Variables|Default|GetDebugTimerDuration)))
      (if (and (Variables|Default|GetDebugCost) (not (.bIsBlocking (Utilities|Struct|BreakHexTile _array_element))))
        (CallFunction|DrawDebugCost (.WorldPosition (Utilities|Struct|BreakHexTile _array_element)) (.Cost (Utilities|Struct|BreakHexTile _array_element)) (Variables|Default|GetDebugTimerDuration) (Utilities|IsValid (.StandingActor (Utilities|Struct|BreakHexTile _array_element))) (.HasAIBooked (Utilities|Struct|BreakHexTile _array_element))))
      (if (Variables|Default|GetDebugRowColumn)
        (CallFunction|DrawDebugRowColumn (.CubeCoord (Utilities|Struct|BreakHexTile _array_element)) (.WorldPosition (Utilities|Struct|BreakHexTile _array_element)) (Variables|Default|GetDebugTimerDuration))))))

(event Custom|On%20Timer%20Tick
  ;[1 1 1] Start the Timer for debug draws
  (CallFunction|EventDebugDraws))

(event EventBeginPlay
  (bind _returnvalue (Game|GetPlayerController 0))
  (bind _cheatmanager (Variables|/Script/Engine.PlayerController|GetCheatManager _returnvalue))
  (Utilities|IsValid _cheatmanager
    (:Is%20Valid
      (bind _asthe_one_cheat_manager (Utilities|Casting|CastToTheOneCheatManager _cheatmanager))
      (if (Class|TheOneCheatManager|IsEnableCheat _asthe_one_cheat_manager)
        ;[1 1 1] Start the Timer for debug draws
        (Utilities|Time|SetTimerbyEvent (delegate Custom|On%20Timer%20Tick) (Variables|Default|GetDebugTimerDuration) true)
        (CallFunction|EventDebugDraws)))))

(event Input|KeyboardEvents|C
  (params (Key :type Key%20Structure))
  ;[1 1 1] Draw tiles Cube Debug
  (:Pressed
    (bind _isa (Utilities|FlowControl|FlipFlop)
      (:A
        _)
      (:B
        _))
    (Variables|Default|SetDebugCost _isa)))

(event Input|KeyboardEvents|R
  (params (Key :type Key%20Structure))
  ;[1 1 1] Draw tiles Cube Debug
  (:Pressed
    (bind _isa (Utilities|FlowControl|FlipFlop)
      (:A
        _)
      (:B
        _))
    (Variables|Default|SetDebugRowColumn _isa)))

(event Input|KeyboardEvents|H
  (params (Key :type Key%20Structure))
  ;[1 1 1] Draw tiles Cube Debug
  (:Pressed
    (bind _isa (Utilities|FlowControl|FlipFlop)
      (:A
        _)
      (:B
        _))
    (Variables|Default|SetDebugCoords _isa)))

(event Input|KeyboardEvents|D
  (params (Key :type Key%20Structure))
  ;[1 1 1] Draw tiles Cube Debug
  (:Pressed
    (bind _isa (Utilities|FlowControl|FlipFlop)
      (:A
        _)
      (:B
        _))
    (Variables|Default|SetDebugCursorPoint _isa)))

(event Input|MouseEvents|RightMouseButton
  (params (Key :type Key%20Structure))
  (:Pressed
    (Default|CallOnRightClickHexGrid (Variables|Default|GetMouseHitRow) (Variables|Default|GetMouseHitColumn) (Variables|Default|GetMouseHitLocation))))

(fn ConstructionScript)

(fn DrawDebugCoords
  (params (H :type H%20Cube%20Coord%20Structure%20%28by%20ref%29) (V :type Vector) (Duration :type Float%20%28double-precision%29))
  (bind _qrs (Utilities|Struct|BreakHCubeCoord H))
  (bind _returnvalue (+ V "-50.000000,0.000000,0.000000"))
  (bind _returnvalue_2 (+ V "50.000000,-50.000000,0.000000"))
  (bind _returnvalue_3 (+ V "50.000000,50.000000,0.000000"))
  (bind (_x _y _z) (Utilities|Struct|BreakIntVector _qrs))
  (LocalVariables|SetDurationLocal Duration)
  (bind _returnvalue_4 (Class|HexGrid|HexEqual H (Utilities|Struct|MakeHCubeCoord "(X=0,Y=0,Z=0)")))
  (if _returnvalue_4
    (Rendering|Debug|DrawDebugString _returnvalue_2 "0" 0 "(R=0.463542,G=0.000000,B=0.027630,A=1.000000)" (LocalVariables|GetDurationLocal))
    (Rendering|Debug|DrawDebugString _returnvalue_3 "0" 0 "(R=0.000000,G=0.079664,B=0.843750,A=1.000000)" (LocalVariables|GetDurationLocal))
    (Rendering|Debug|DrawDebugString _returnvalue "0" 0 "(R=0.000000,G=1.000000,B=0.020103,A=1.000000)" (LocalVariables|GetDurationLocal))
    (else
      (Rendering|Debug|DrawDebugString _returnvalue_2 (Utilities|String|ToString(Integer) _x) 0 "(R=0.462077,G=0.000000,B=0.027321,A=1.000000)" (LocalVariables|GetDurationLocal))
      (Rendering|Debug|DrawDebugString _returnvalue_3 (Utilities|String|ToString(Integer) _y) 0 "(R=0.000000,G=0.080220,B=0.846873,A=1.000000)" (LocalVariables|GetDurationLocal))
      (Rendering|Debug|DrawDebugString _returnvalue (Utilities|String|ToString(Integer) _z) 0 "(R=0.000000,G=1.000000,B=0.020289,A=1.000000)" (LocalVariables|GetDurationLocal)))))

(fn DrawDebugCost
  (params (V :type Vector) (C :type Float%20%28double-precision%29) (Duration :type Float%20%28double-precision%29) (HasAI :type Boolean) (HasBooked :type Boolean))
  (Rendering|Debug|DrawDebugString V (Utilities|String|ToString(Text) (Utilities|Text|ToText(Float) C "HalfToEven")) 0 "(R=1.000000,G=1.000000,B=1.000000,A=1.000000)" Duration)
  (Rendering|Debug|DrawDebugString (+ V "50.000000,0.000000,0.000000") (Utilities|String|ToString(Text) (Utilities|Text|FormatText "Has:{HasAI}" HasAI)) 0 "(R=1.000000,G=1.000000,B=1.000000,A=1.000000)" Duration)
  (Rendering|Debug|DrawDebugString (+ V "100.000000,0.000000,0.000000") (Utilities|String|ToString(Text) (Utilities|Text|FormatText "Bk:{BKDI}" HasBooked)) 0 "(R=1.000000,G=1.000000,B=1.000000,A=1.000000)" Duration))

(fn DrawDebugRowColumn
  (params (H :type H%20Cube%20Coord%20Structure) (V :type Vector) (Duration :type Float%20%28double-precision%29))
  (bind _qrs (Utilities|Struct|BreakHCubeCoord H))
  (bind _tileconfig (Variables|Default|GetTileConfig))
  (bind (_tileorientation _tilesize _origin _baseonradius) (Utilities|Struct|BreakHTileConfig _tileconfig))
  (if (not _baseonradius)
    (LocalVariables|SetTextLocation (+ V "0.000000,-50.000000,20.000000"))
    (LocalVariables|SetLocalDuration Duration)
    (switch Utilities|FlowControl|Switch|SwitchonEHTileOrientationFlag _tileorientation
      (:FLAT
        (Rendering|Debug|DrawDebugString (LocalVariables|GetTextLocation) (Utilities|String|ToString(Text) (Utilities|Text|FormatText "(R:{Row}, C:{Column})" (+ (.y _qrs) (/ (- (.x _qrs) (Class|KismetMathLibrary|AndIntInt (.x _qrs) 1)) 2)) (.x _qrs))) 0 "(R=1.000000,G=1.000000,B=1.000000,A=1.000000)" (LocalVariables|GetLocalDuration)))
      (:POINTY
        (Rendering|Debug|DrawDebugString (LocalVariables|GetTextLocation) (Utilities|String|ToString(Text) (Utilities|Text|FormatText "(R:{Row}, C:{Column})" (.y _qrs) (+ (.x _qrs) (/ (- (.y _qrs) (Class|KismetMathLibrary|AndIntInt (.y _qrs) 1)) 2)))) 0 "(R=1.000000,G=1.000000,B=1.000000,A=1.000000)" (LocalVariables|GetLocalDuration))))))