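; Default Gameplay Ability that plays its AbilityMontage and triggers tagged actions at points during it.
; Once the montage task starts, six parallel event listeners on the ActionPoint0–5 tags each pass their tag to DoAction every time they fire.
; The ability ends when the montage completes, is interrupted or is cancelled, or immediately when no valid montage is set.
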(event Ability|EventActivateAbility
  (Utilities|IsValid (Variables|Default|GetAbilityMontage)
    (:Is%20Valid
      (|PlayMontageandWaitProxy "None" (Variables|Default|GetAbilityMontage) 1.0 "None" true 1.0 0.0 false
        (:then
          (Utilities|FlowControl|Sequence
            (:then_0
              (|MontagePost "(TagName=\"Ability.ActionPoint0\")" false
                (:EventReceived
                  (Class|TheOneGeneralGA|DoAction "(TagName=\"Ability.ActionPoint0\")"))))
            (:then_1
              (|MontagePost "(TagName=\"Ability.ActionPoint1\")" false
                (:EventReceived
                  (Class|TheOneGeneralGA|DoAction "(TagName=\"Ability.ActionPoint1\")"))))
            (:then_2
              (|MontagePost "(TagName=\"Ability.ActionPoint2\")" false
                (:EventReceived
                  (Class|TheOneGeneralGA|DoAction "(TagName=\"Ability.ActionPoint2\")"))))
            (:then_3
              (|MontagePost "(TagName=\"Ability.ActionPoint3\")" false
                (:EventReceived
                  (Class|TheOneGeneralGA|DoAction "(TagName=\"Ability.ActionPoint3\")"))))
            (:then_4
              (|MontagePost "(TagName=\"Ability.ActionPoint4\")" false
                (:EventReceived
                  (Class|TheOneGeneralGA|DoAction "(TagName=\"Ability.ActionPoint4\")"))))
            (:then_5
              (|MontagePost "(TagName=\"Ability.ActionPoint5\")" false
                (:EventReceived
                  (Class|TheOneGeneralGA|DoAction "(TagName=\"Ability.ActionPoint5\")"))))))
        (:OnCompleted
          (Ability|EndAbility :!label _label))
        (:OnInterrupted
          (goto _label))
        (:OnCancelled
          (goto _label))))
    (:Is%20Not%20Valid
      (Ability|EndAbility))))

(event Ability|EventOnEndAbility
  (params (bWasCancelled :type Boolean)))