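; Default attack Gameplay Ability that plays an attack montage and fires timed attack points during it.
; An AttackSpeed value from the ability system, treated as a duration, scales the montage rate and places a timer at each AttackPointPercents fraction.
; Each attack point increments a counter and calls NativeOnAttackPoint, flagging the last one.
; The ability ends when the montage completes or cancels, and ending clears all timers.
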(event Custom|Event%20AttackPoint
  (bind _output_get (Variables|Default|SetTempPassedAttackPoint (+ (Variables|Default|GetTempPassedAttackPoint) 1)))
  (Class|TheOneAttackGA|NativeonAttackPoint (== _output_get (Utilities|Array|Length (Variables|Default|GetAttackPointPercents)))))

(event Ability|EventActivateAbility
  (Variables|Default|SetTempPassedAttackPoint 0)
  (Variables|Default|SetAttackSpeed (.ReturnValue (Ability|Attribute|GetFloatAttributefromAbilitySystemComponent (Ability|GetAbilitySystemComponentfromActorInfo) "(AttributeName=\"AttackSpeed\",Attribute=/Script/TheOne.TheOneAttributeSet:AttackSpeed,AttributeOwner=\"/Script/CoreUObject.Class'/Script/TheOne.TheOneAttributeSet'\")")))
  (|PlayMontageandWaitProxy "None" (Variables|Default|GetAbilityMontage) (/ (Variables|Default|GetNormalizeRate) (Variables|Default|GetAttackSpeed)) "None" true 1.0 0.0 false
    (:then
      (for _array_element (Variables|Default|GetAttackPointPercents)
        (bind _returnvalue (Utilities|Time|SetTimerbyEvent (EventDispatchers|CreateEvent :!event Custom|Event%20AttackPoint) (* (Variables|Default|GetAttackSpeed) _array_element) false true))
        (Utilities|Array|Add (Variables|Default|GetAttackHandles) _returnvalue)))
    (:OnCompleted
      (Ability|EndAbility :!label _label))
    (:OnCancelled
      (goto _label))))

(event Ability|EventOnEndAbility
  (params (bWasCancelled :type Boolean))
  (for _array_element (Variables|Default|GetAttackHandles)
    (Utilities|Time|ClearandInvalidateTimerbyHandle _array_element))
  (Utilities|Array|Clear (Variables|Default|GetAttackHandles)))