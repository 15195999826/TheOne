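; Gameplay ability for data-driven passives that react to battle events by playing queued montages and running their actions.
; On activation it listens for battle event payloads, which ReceiveBattleEvent turns into a list of event IDs.
; Starting next tick, a recursive loop plays each ID's mapped montage, with ActionPoint tag listeners calling ExecuteMontageAction.
; Listeners end when each montage completes or aborts, and an empty queue calls ExecuteOver.
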(event Custom|Event%20Play%20Montage%20Loop
  (Variables|Default|SetCurrentPlayingEventID (Utilities|Array|Get(acopy) (Variables|Default|GetTempToPlayMontageEvnets)))
  (|PlayMontageandWaitProxy "None" (.Value (Utilities|Map|Find (Variables|Default|GetEventID2MontageMap) (Variables|Default|GetCurrentPlayingEventID))) 1.0 "None" true 1.0 0.0 false
    (:then
      (Utilities|Array|RemoveIndex (Variables|Default|GetTempToPlayMontageEvnets))
      (Utilities|FlowControl|Sequence
        (:then_0
          (bind _asynctaskproxy (|MontagePost "(TagName=\"Ability.ActionPoint0\")" false)
            (:then
              (Utilities|Array|Add (Variables|Default|GetMontagePostTasks) _asynctaskproxy))
            (:EventReceived
              (Class|TheOneDataDrivePassiveGA|ExecuteMontageAction (Variables|Default|GetCurrentPlayingEventID) "(TagName=\"Ability.ActionPoint0\")"))))
        (:then_1
          (bind _asynctaskproxy_2 (|MontagePost "(TagName=\"Ability.ActionPoint1\")" false)
            (:then
              (Utilities|Array|Add (Variables|Default|GetMontagePostTasks) _asynctaskproxy_2))
            (:EventReceived
              (Class|TheOneDataDrivePassiveGA|ExecuteMontageAction (Variables|Default|GetCurrentPlayingEventID) "(TagName=\"Ability.ActionPoint1\")"))))
        (:then_2
          (bind _asynctaskproxy_3 (|MontagePost "(TagName=\"Ability.ActionPoint2\")" false)
            (:then
              (Utilities|Array|Add (Variables|Default|GetMontagePostTasks) _asynctaskproxy_3))
            (:EventReceived
              (Class|TheOneDataDrivePassiveGA|ExecuteMontageAction (Variables|Default|GetCurrentPlayingEventID) "(TagName=\"Ability.ActionPoint2\")"))))
        (:then_3
          (bind _asynctaskproxy_4 (|MontagePost "(TagName=\"Ability.ActionPoint3\")" false)
            (:then
              (Utilities|Array|Add (Variables|Default|GetMontagePostTasks) _asynctaskproxy_4))
            (:EventReceived
              (Class|TheOneDataDrivePassiveGA|ExecuteMontageAction (Variables|Default|GetCurrentPlayingEventID) "(TagName=\"Ability.ActionPoint3\")"))))
        (:then_4
          (bind _asynctaskproxy_5 (|MontagePost "(TagName=\"Ability.ActionPoint4\")" false)
            (:then
              (Utilities|Array|Add (Variables|Default|GetMontagePostTasks) _asynctaskproxy_5))
            (:EventReceived
              (Class|TheOneDataDrivePassiveGA|ExecuteMontageAction (Variables|Default|GetCurrentPlayingEventID) "(TagName=\"Ability.ActionPoint4\")"))))
        (:then_5
          (bind _asynctaskproxy_6 (|MontagePost "(TagName=\"Ability.ActionPoint5\")" false)
            (:then
              (Utilities|Array|Add (Variables|Default|GetMontagePostTasks) _asynctaskproxy_6))
            (:EventReceived
              (Class|TheOneDataDrivePassiveGA|ExecuteMontageAction (Variables|Default|GetCurrentPlayingEventID) "(TagName=\"Ability.ActionPoint5\")"))))))
    (:OnCompleted
      (for _array_element (Variables|Default|GetMontagePostTasks) :!label _label
        (Utilities|IsValid _array_element
          (:Is%20Valid
            (GameplayTasks|EndTask _array_element))))
      (Utilities|Array|Clear (Variables|Default|GetMontagePostTasks))
      (if (> (Utilities|Array|Length (Variables|Default|GetTempToPlayMontageEvnets)) 0)
        (CallFunction|EventPlayMontageLoop)
        (else
          (CallFunction|GetMontagesOver))))
    (:OnInterrupted
      (goto _label))
    (:OnCancelled
      (goto _label))))

(event Custom|Get%20Montages%20Over
  (Class|TheOneDataDrivePassiveGA|ExecuteOver))

(event Ability|EventActivateAbility
  (bind _payload (|TheOneBattleEventPak)
    (:EventReceived
      (bind _returnvalue (Class|TheOneDataDrivePassiveGA|ReceiveBattleEvent _payload))
      (bind _output_get (Variables|Default|SetTempToPlayMontageEvnets _returnvalue))
      (if (> (Utilities|Array|Length _output_get) 0)
        (EventDispatchers|BindEventtoOnMontagesOver (EventDispatchers|CreateEvent :!event Custom|Get%20Montages%20Over))
        (Utilities|FlowControl|DelayUntilNextTick)
        (CallFunction|EventPlayMontageLoop)
        (else
          (CallFunction|GetMontagesOver))))))

(event Ability|EventOnEndAbility
  (params (bWasCancelled :type Boolean)))