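; AI controller for Battle Chess that starts BT_BattleChessAI on BeginPlay and turns committed commands into blackboard quests.
; CommitAbility clears the have-quest flag, then maps move, item or weapon-ability commands to quest type, target and payload keys.
; The flag is set again only after those keys are written; Invalid commands leave it cleared.
; SetAITargetActor and SetAITargetLocation are empty, with older targeting logic left disconnected.
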(event EventBeginPlay
  (|CallParentFunction)
  (AI|RunBehaviorTree "/Game/Blueprints/AI/BattleChessAI/BT_BattleChessAI.BT_BattleChessAI"))

(event EventTick
  (params (DeltaSeconds :type Float%20%28single-precision%29)))

(event EventSetAITargetLocation
  (params (Location :type Vector%20%28by%20ref%29 :default "0, 0, 0")))

(event EventSetAITargetActor
  (params (TargetActor :type Actor%20Object%20Reference)))

(event EventCommitAbility
  (params (Payload :type The%20One%20Use%20Ability%20Command%20Payload%20Structure) (InTargetActor :type Actor%20Object%20Reference) (InLocation :type Vector%20%28by%20ref%29 :default "0, 0, 0") (InReleaseDistance :type Integer))
  (bind (_commandtype _intpayload _vectorpayload) (Utilities|Struct|BreakTheOneUseAbilityCommandPayload Payload))
  (AI|Components|Blackboard|SetValueasBool (Variables|Default|GetBlackboardComponent) (Variables|Default|GetHaveQuestKey) false)
  (switch Utilities|FlowControl|Switch|SwitchonETheOneUseAbilityCommandType _commandtype
    (:Invalid
      (AI|Components|Blackboard|SetValueasEnum (Variables|Default|GetBlackboardComponent) (Variables|Default|GetQuestTypeKey)))
    (:UseItem
      (AI|Components|Blackboard|SetValueasEnum (Variables|Default|GetBlackboardComponent) (Variables|Default|GetQuestTypeKey) 4)
      (AI|Components|Blackboard|SetValueasObject (Variables|Default|GetBlackboardComponent) (Variables|Default|GetTargetActorKey) InTargetActor :!label _label)
      (AI|Components|Blackboard|SetValueasVector (Variables|Default|GetBlackboardComponent) (Variables|Default|GetTargetLocation) InLocation)
      (Class|BlackboardComponent|SetValueasInt (Variables|Default|GetBlackboardComponent) (Variables|Default|GetGoalDistanceKey) InReleaseDistance)
      (Class|BlackboardComponent|SetValueasInt (Variables|Default|GetBlackboardComponent) (Variables|Default|GetAbilityPayloadKey) _intpayload)
      (AI|Components|Blackboard|SetValueasBool (Variables|Default|GetBlackboardComponent) (Variables|Default|GetHaveQuestKey) true))
    (:UseWeaponAbility
      (AI|Components|Blackboard|SetValueasEnum (Variables|Default|GetBlackboardComponent) (Variables|Default|GetQuestTypeKey) 3)
      (goto _label))
    (:Move
      (AI|Components|Blackboard|SetValueasVector (Variables|Default|GetBlackboardComponent) (Variables|Default|GetTargetLocation) _vectorpayload)
      (Class|BlackboardComponent|SetValueasInt (Variables|Default|GetBlackboardComponent) (Variables|Default|GetGoalDistanceKey))
      (AI|Components|Blackboard|SetValueasEnum (Variables|Default|GetBlackboardComponent) (Variables|Default|GetQuestTypeKey) 1)
      (AI|Components|Blackboard|SetValueasBool (Variables|Default|GetBlackboardComponent) (Variables|Default|GetHaveQuestKey) true))))

(fn ConstructionScript)