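; Behavior Tree task for debugging that prints the controlled pawn's name when it executes or aborts.
; Each tick increments CurrentTick, and once it exceeds TickCount the task prints DebugText and finishes with success.
; The graph never resets CurrentTick or calls FinishAbort, and a per-tick name print is left unconnected.
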(event EventReceiveExecuteAI
  (params (OwnerController :type AI%20Controller%20Object%20Reference) (ControlledPawn :type Pawn%20Object%20Reference))
  (Development|PrintString (Utilities|String|ToString(Text) (Utilities|Text|FormatText "{Name} Execute AI" (Utilities|GetDisplayName ControlledPawn)))))

(event EventReceiveAbortAI
  (params (OwnerController :type AI%20Controller%20Object%20Reference) (ControlledPawn :type Pawn%20Object%20Reference))
  (Development|PrintString (Utilities|String|ToString(Text) (Utilities|Text|FormatText "{Name}  Abort AI" (Utilities|GetDisplayName ControlledPawn)))))

(event EventReceiveTickAI
  (params (OwnerController :type AI%20Controller%20Object%20Reference) (ControlledPawn :type Pawn%20Object%20Reference) (DeltaSeconds :type Float%20%28single-precision%29))
  (Variables|Default|SetCurrentTick (+ (Variables|Default|GetCurrentTick) 1))
  (if (> (Variables|Default|GetCurrentTick) (Variables|Default|GetTickCount))
    (Development|PrintString (Variables|Default|GetDebugText))
    (AI|BehaviorTree|FinishExecute (Variables|Default|GetSuccess))))