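; AI controller for Auto Chess characters that runs the BT_AutoChessAI behavior tree and turns commands into blackboard quests.
; Location, target-actor and ability/item events each write quest type, target and goal distance keys, then set the have-quest flag.
; Actor goal distance comes from a character float attribute; re-sending the same target only prints a debug string.
; Ability commits clear the flag first, so an invalid command leaves no active quest.
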(event EventBeginPlay
  (|CallParentFunction)
  (AI|RunBehaviorTree "/Game/Blueprints/AI/AutoChessAI/BT_AutoChessAI.BT_AutoChessAI"))

(event EventTick
  (params (DeltaSeconds :type Float%20%28single-precision%29)))

(event EventSetAITargetLocation
  (params (Location :type Vector%20%28by%20ref%29 :default "0, 0, 0"))
  (AI|Components|Blackboard|SetValueasVector (Variables|Default|GetBlackboardComponent) (Variables|Default|GetTargetLocation) Location)
  (AI|Components|Blackboard|SetValueasObject (Variables|Default|GetBlackboardComponent) (Variables|Default|GetTargetActorKey) 0)
  (Class|BlackboardComponent|SetValueasInt (Variables|Default|GetBlackboardComponent) (Variables|Default|GetGoalDistanceKey))
  (AI|Components|Blackboard|SetValueasEnum (Variables|Default|GetBlackboardComponent) (Variables|Default|GetQuestTypeKey) 1)
  (AI|Components|Blackboard|SetValueasBool (Variables|Default|GetBlackboardComponent) (Variables|Default|GetHaveQuestKey) true))

(event EventSetAITargetActor
  (params (TargetActor :type Actor%20Object%20Reference))
  (if (== TargetActor (AI|Components|Blackboard|GetValueasObject (Variables|Default|GetBlackboardComponent) (Variables|Default|GetTargetActorKey)))
    (Development|PrintString "Hello")
    (else
      (AI|Components|Blackboard|SetValueasObject (Variables|Default|GetBlackboardComponent) (Variables|Default|GetTargetActorKey) TargetActor)
      (Class|BlackboardComponent|SetValueasInt (Variables|Default|GetBlackboardComponent) (Variables|Default|GetGoalDistanceKey) (Math|Float|Truncate (.ReturnValue (Ability|Attribute|GetFloatAttribute (Variables|Default|GetWeakTheOneCharacterBase) "(AttributeName=\"AttackRange\",Attribute=/Script/TheOne.TheOneAttributeSet:AttackRange,AttributeOwner=\"/Script/CoreUObject.Class'/Script/TheOne.TheOneAttributeSet'\")"))))
      (AI|Components|Blackboard|SetValueasEnum (Variables|Default|GetBlackboardComponent) (Variables|Default|GetQuestTypeKey) 2)
      (AI|Components|Blackboard|SetValueasBool (Variables|Default|GetBlackboardComponent) (Variables|Default|GetHaveQuestKey) true))))

(event EventCommitAbility
  (params (Payload :type The%20One%20Use%20Ability%20Command%20Payload%20Structure) (InTargetActor :type Actor%20Object%20Reference) (InLocation :type Vector%20%28by%20ref%29 :default "0, 0, 0") (InReleaseDistance :type Integer))
  (bind (_commandtype _intpayload) (Utilities|Struct|BreakTheOneUseAbilityCommandPayload Payload))
  (AI|Components|Blackboard|SetValueasBool (Variables|Default|GetBlackboardComponent) (Variables|Default|GetHaveQuestKey) false)
  (switch Utilities|FlowControl|Switch|SwitchonETheOneUseAbilityCommandType _commandtype
    (:Invalid
      (AI|Components|Blackboard|SetValueasEnum (Variables|Default|GetBlackboardComponent) (Variables|Default|GetQuestTypeKey)))
    (:UseItem
      (AI|Components|Blackboard|SetValueasEnum (Variables|Default|GetBlackboardComponent) (Variables|Default|GetQuestTypeKey) 4)
      (AI|Components|Blackboard|SetValueasObject (Variables|Default|GetBlackboardComponent) (Variables|Default|GetTargetActorKey) InTargetActor :!label _label)
      (AI|Components|Blackboard|SetValueasVector (Variables|Default|GetBlackboardComponent) (Variables|Default|GetTargetLocation) InLocation)
      (Class|BlackboardComponent|SetValueasInt (Variables|Default|GetBlackboardComponent) (Variables|Default|GetGoalDistanceKey) InReleaseDistance)
      (Class|BlackboardComponent|SetValueasInt (Variables|Default|GetBlackboardComponent) (Variables|Default|GetAbilityPayloadKey) _intpayload)
      (AI|Components|Blackboard|SetValueasBool (Variables|Default|GetBlackboardComponent) (Variables|Default|GetHaveQuestKey) true))
    (:UseWeaponAbility
      (AI|Components|Blackboard|SetValueasEnum (Variables|Default|GetBlackboardComponent) (Variables|Default|GetQuestTypeKey) 3)
      (goto _label))))

(fn ConstructionScript)